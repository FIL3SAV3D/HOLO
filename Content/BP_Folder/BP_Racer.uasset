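; Player-controlled hover racer pawn that follows the ground surface beneath it.
; Each Tick, forward-offset line traces set hover height and interpolate rotation to the surface normal, falling by Gravity and leveling when nothing is hit.
; Axis inputs add physics velocity for thrust and boost and torque for steering, while thrust spins RacerCore and velocity widens the camera FOV.
; Possession adds the WB_Speed widget to the viewport.
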(event EventBeginPlay)

(event Collision|EventActorBeginOverlap
  (params (OtherActor :type Actor%20Object%20Reference)))

(event EventTick
  (params (DeltaSeconds :type Float%20%28single-precision%29))
  (bind _returnvalue (Utilities|Time|GetWorldDeltaSeconds))
  (bind _returnvalue_2 (Transformation|GetActorLocation))
  (bind (_actorlocation _actorupvector _actorrightvector _actorforwardvector) (CallFunction|GetActorLocation&Rotation))
  (bind _returnvalue_3 (Transformation|GetActorRotation))
  (bind (_x _y _z) (Math|Vector|BreakVector _returnvalue_2))
  (bind _returnvalue_4 (* _actorforwardvector 3e+02))
  (bind (_hitnormal _returnvalue_5 _impactpoint) (CallFunction|LineTraceGround (+ _returnvalue_4 _actorlocation) (+ _returnvalue_4 (- _actorlocation (* _actorupvector (Variables|Default|GetHoverHeight)))) "(R=1.000000,G=0.000000,B=0.033492,A=1.000000)")) ; GroundTraceForLocation
  (Transformation|SetActorLocation (select (< (Math|Vector|Distance(Vector) (Math|Interpolation|VInterpTo (Transformation|GetActorLocation) (Math|Vector|SelectVector (+ (* (Transformation|GetActorUpVector) (/ (Variables|Default|GetHoverHeight) 2.0)) (- _impactpoint (* (Transformation|GetActorForwardVector) 3e+02))) (Math|Vector|MakeVector _x _y (- _z (Variables|Default|GetGravity))) _returnvalue_5) _returnvalue 1e+02) (- _impactpoint (* (Transformation|GetActorForwardVector) 3e+02))) 3.5e+02) (- (Math|Vector|SelectVector (+ (* (Transformation|GetActorUpVector) (/ (Variables|Default|GetHoverHeight) 2.0)) (- _impactpoint (* (Transformation|GetActorForwardVector) 3e+02))) (Math|Vector|MakeVector _x _y (- _z (Variables|Default|GetGravity))) _returnvalue_5) (* (Transformation|GetActorUpVector) 5e+01)) (Math|Interpolation|VInterpTo (Transformation|GetActorLocation) (Math|Vector|SelectVector (+ (* (Transformation|GetActorUpVector) (/ (Variables|Default|GetHoverHeight) 2.0)) (- _impactpoint (* (Transformation|GetActorForwardVector) 3e+02))) (Math|Vector|MakeVector _x _y (- _z (Variables|Default|GetGravity))) _returnvalue_5) _returnvalue 1e+02)) false false)
  (bind (_hitnormal_2 _returnvalue_6) (CallFunction|LineTraceGround (+ (* _actorforwardvector (Variables|Default|GetOffset)) _actorlocation) (+ (- _actorlocation (* _actorupvector (Variables|Default|GetHoverHeight))) (* _actorforwardvector (+ (Variables|Default|GetOffset) 3e+02))) "(R=0.955539,G=1.000000,B=0.000000,A=1.000000)")) ; GroundTraceForRotation
  (Transformation|SetWorldRotation (Variables|Default|GetRacerTop) (Math|Interpolation|RInterpTo _returnvalue_3 (select _returnvalue_6 (Math|Rotator|MakeRotationfromAxes (Math|Vector|CrossProduct _actorrightvector _hitnormal_2) _actorrightvector _hitnormal_2) (Math|Rotator|MakeRotator 0.0 0.0 (.Yaw (Math|Rotator|BreakRotator _returnvalue_3)))) _returnvalue 2e+01) false false))

(event EventPossessed
  (params (NewController :type Controller%20Object%20Reference))
  (bind _returnvalue (UserInterface|CreateWidget "/Game/UI/WB_Folder/WB_Speed.WB_Speed_C"))
  (UserInterface|Viewport|AddtoViewport _returnvalue 0))

(event Input|AxisEvents|InputAxisForwardBackward
  (params (AxisValue :type Float%20%28single-precision%29))
  (bind _returnvalue (Utilities|Time|GetWorldDeltaSeconds))
  (bind _returnvalue_2 (Transformation|GetActorForwardVector))
  (bind _returnvalue_3 (Transformation|GetActorLocation))
  (bind _returnvalue_4 (Transformation|GetActorForwardVector))
  (bind _boost (Variables|Default|GetBoost))
  (bind _forwardforce (Variables|Default|GetForwardForce))
  (bind _returnvalue_5 (* AxisValue _forwardforce))
  (bind _returnvalue_6 (* _returnvalue_2 _boost))
  (bind _returnvalue_7 (* _returnvalue_4 _returnvalue_5))
  (bind _returnvalue_8 (+ _returnvalue_7 _returnvalue_6))
  (bind _returnvalue_9 (* _returnvalue_8 1e+02))
  (bind _returnvalue_10 (* _returnvalue _returnvalue_9))
  (Physics|SetPhysicsLinearVelocity (Variables|Default|GetRacerTop) _returnvalue_10 true "None")
  (CallFunction|LineTraceGround _returnvalue_3 (+ _returnvalue_3 _returnvalue_10))
  (Transformation|AddLocalRotation (Variables|Default|GetRacerCore) (Math|Rotator|MakeRotator 0.0 (Math|Float|MapRangeClamped (Math|Vector|VectorLength _returnvalue_10) 0.0 1.5e+03 -1e+01 -1e+04) 0.0) false false)
  (bind _returnvalue_11 (Physics|GetPhysicsLinearVelocity (Variables|Default|GetRacerTop) "None"))
  (Camera|SetFieldOfView (Variables|Default|GetCamera) (+ (Math|Float|MapRangeClamped (/ (Math|Vector|VectorLength _returnvalue_11) 1e+03) 0.0 6e+01 3e+01 7e+01) 6e+01)))

(event Input|AxisEvents|InputAxisTurnLeftRight
  (params (AxisValue :type Float%20%28single-precision%29))
  (Class|PrimitiveComponent|AddTorqueinRadians (Variables|Default|GetRacerTop) (Math|Vector|Lerp(Vector) "0, 0, 0" (* (Transformation|GetActorUpVector) (* AxisValue (Variables|Default|GetZ%20%28Yaw%29))) 0.4) "None" true))

(event Input|AxisEvents|InputAxisBoost
  (params (AxisValue :type Float%20%28single-precision%29))
  (Variables|Default|SetBoost (* AxisValue 5e+02)))

(fn ConstructionScript)

(fn TraceGroundMidPoint
  (bind _returnvalue (Transformation|GetActorLocation))
  (bind (_outhit _returnvalue_2) (Collision|LineTraceByChannel _returnvalue (+ _returnvalue (Math|Vector|MakeVector 0.0 0.0 (* (Variables|Default|GetHoverHeight) -2.0))) "TraceTypeQuery2" true 0 "ForOneFrame"))
  (if _returnvalue_2
    (return (.Distance (Collision|BreakHitResult _outhit)))
    (else
      (return (.Distance (Collision|BreakHitResult _outhit))))))

(fn LineTraceGround
  (params (Start :type Vector) (End :type Vector) (TraceColor :type Linear%20Color%20Structure))
  (bind (_outhit _returnvalue) (Collision|LineTraceByChannel Start End "TraceTypeQuery1" true 0 "ForOneFrame" true TraceColor))
  (return (.Normal (Collision|BreakHitResult _outhit)) _returnvalue (.ImpactPoint (Collision|BreakHitResult _outhit)) (.PhysMat (Collision|BreakHitResult _outhit))))

(fn GetActorLocation&Rotation
  (bind _returnvalue (Transformation|GetActorRotation))
  (return (Transformation|GetActorLocation) (Math|Vector|GetUpVector _returnvalue) (Math|Vector|GetRightVector _returnvalue) (Math|Vector|GetForwardVector _returnvalue)))

(fn DebugTracer
  (params (InVector :type Vector))
  (bind _returnvalue (Transformation|GetActorLocation))
  (CallFunction|LineTraceGround _returnvalue (+ _returnvalue InVector) "(R=1.000000,G=0.000000,B=0.162540,A=1.000000)")
  (return))